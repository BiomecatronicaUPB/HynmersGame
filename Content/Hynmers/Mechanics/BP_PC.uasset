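; BP_PC is an interactable PC actor that starts a navigation series on its parent BP_Nav actor.
; A looping timeline starts on BeginPlay and drives the point light intensity in a breathing pulse.
; On Interact, it casts its parent actor to BP_Nav, passes the interacting pawn to StartNavSerie, then stops the light animation.
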(event EventBeginPlay
  (Components|Timeline|SetLooping (Variables|Default|GetLight_Animation) true)
  (bind _beathing_light (Timeline|Light_Animation Play)
    (:Update
      (Rendering|Components|Light|SetIntensity (Variables|Default|GetPointLight) _beathing_light))))

(event Collision|EventActorBeginOverlap
  (params (OtherActor :type Actor%20Object%20Reference)))

(event EventTick
  (params (DeltaSeconds :type Float%20%28single-precision%29)))

(event EventInteract
  (params (InteractionPawn :type Pawn%20Object%20Reference))
  (bind _asbp_nav (Utilities|Casting|CastToBP_Nav (Actor|GetParentActor)))
  (Default|StartNavSerie _asbp_nav InteractionPawn)
  (Audio|Components|Audio|Stop (Variables|Default|GetLight_Animation)))

(fn ConstructionScript)