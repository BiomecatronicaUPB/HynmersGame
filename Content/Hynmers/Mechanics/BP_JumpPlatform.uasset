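; BP_JumpPlatform is a jump platform that can be shown or hidden and reports pawn landings to its parent BP_Lab.
; On BeginPlay it makes its Collisions component hierarchy invisible and uses AdjacentFinder overlaps to cache other platforms in the same Zone as neighbors.
; When PawnLanded fires, it hides itself and passes those neighbors to the parent lab's ShowNextHexagon.
; Show and Hide only toggle visibility and hidden-in-game state.
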(event Custom|PawnLanded
  (CallFunction|Hide)
  (bind _asbp_lab (Utilities|Casting|CastToBP_Lab (Actor|GetParentActor)))
  (Default|ShowNextHexagon _asbp_lab (Variables|Default|GetAdjacentJumpPlatforms)))

(event Custom|Hide
  (bind _collisions (Variables|Default|GetCollisions))
  (Rendering|SetVisibility _collisions false true)
  (Development|SetHiddeninGame _collisions true true))

(event Custom|Show
  (bind _collisions (Variables|Default|GetCollisions))
  (Rendering|SetVisibility _collisions true true)
  (Development|SetHiddeninGame _collisions false true))

(event EventBeginPlay
  (Rendering|SetVisibility (Variables|Default|GetCollisions) false true)
  (for _array_element (Collision|GetOverlappingActors (Variables|Default|GetAdjacentFinder) "BP_JumpPlatform_C" :!class /Script/Engine.PrimitiveComponent)
    (bind _asbp_jump_platform (Utilities|Casting|CastToBP_JumpPlatform _array_element))
    (if (== (Variables|BP_JumpPlatform_C|GetZone _asbp_jump_platform) (Variables|Default|GetZone))
      (if (!= _asbp_jump_platform self)
        (Utilities|Array|Add (Variables|Default|GetAdjacentJumpPlatforms) _asbp_jump_platform)))))

(event EventTick
  (params (DeltaSeconds :type Float%20%28single-precision%29)))

(fn ConstructionScript)