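; Elevator actor for the ship map that a pawn operates through Interact, with a swinging door and travel between an upper and lower height.
; Outside and Inside overlap checks decide the action: outside toggles the door, while inside with it open closes it and, after a delay, starts travel.
; Two timelines drive door yaw and actor height in both directions.
; IsActive blocks input effects during travel, and the door reopens on arrival.
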(event Custom|MoveElevatorDown
  (bind _returnvalue (Transformation|GetActorLocation))
  (Utilities|FlowControl|Delay 1.8)
  (if (Variables|Default|GetIsActive)
    (Variables|Default|SetIsActive false)
    (bind _locationpercentage (Timeline|Movement PlayFromStart)
      (:Update
        (Transformation|SetActorLocation (Math|Vector|MakeVector (.x _returnvalue) (.y _returnvalue) (+ (Variables|Default|GetUpLocation) (* _locationpercentage (- (Variables|Default|GetDownLocation) (Variables|Default|GetUpLocation))))) false false))
      (:Finished
        (Variables|Default|SetIsActive true)
        (Variables|Default|SetIsUp (not (Variables|Default|GetIsUp)))
        (CallFunction|OpenDoor)))))

(event Custom|OpenDoor
  (if (Variables|Default|GetIsActive)
    (bind _rotationpercentage (Timeline|DoorMovement Play)
      (:Update
        (Transformation|SetRelativeRotation (Variables|Default|GetDoor) (Math|Rotator|MakeRotator 0.0 0.0 (* _rotationpercentage (Variables|Default|GetLimitRotation))) false false))
      (:Finished
        (Variables|Default|SetIsOpen (not (Variables|Default|GetIsOpen)))))))

(event Custom|CloseDoor
  (if (Variables|Default|GetIsActive)
    (bind _rotationpercentage (Timeline|DoorMovement Reverse)
      (:Update
        (Transformation|SetRelativeRotation (Variables|Default|GetDoor) (Math|Rotator|MakeRotator 0.0 0.0 (* _rotationpercentage (Variables|Default|GetLimitRotation))) false false))
      (:Finished
        (Variables|Default|SetIsOpen (not (Variables|Default|GetIsOpen)))))))

(event Custom|MoveElevatorUp
  (bind _returnvalue (Transformation|GetActorLocation))
  (Utilities|FlowControl|Delay 1.8)
  (if (Variables|Default|GetIsActive)
    (Variables|Default|SetIsActive false)
    (bind _locationpercentage (Timeline|Movement ReverseFromEnd)
      (:Update
        (Transformation|SetActorLocation (Math|Vector|MakeVector (.x _returnvalue) (.y _returnvalue) (+ (Variables|Default|GetUpLocation) (* _locationpercentage (- (Variables|Default|GetDownLocation) (Variables|Default|GetUpLocation))))) false false))
      (:Finished
        (Variables|Default|SetIsActive true)
        (Variables|Default|SetIsUp (not (Variables|Default|GetIsUp)))
        (CallFunction|OpenDoor)))))

(event EventBeginPlay)

(event Collision|EventActorBeginOverlap
  (params (OtherActor :type Actor%20Object%20Reference)))

(event EventTick
  (params (DeltaSeconds :type Float%20%28single-precision%29)))

(event EventInteract
  (params (InteractionPawn :type Pawn%20Object%20Reference))
  (if (Collision|IsOverlappingActor (Variables|Default|GetOutside) InteractionPawn :!class /Script/Engine.PrimitiveComponent)
    (if (Variables|Default|GetIsOpen)
      (CallFunction|CloseDoor)
      (else
        (CallFunction|OpenDoor)))
    (elif (Collision|IsOverlappingActor (Variables|Default|GetInside) InteractionPawn :!class /Script/Engine.PrimitiveComponent)
      (if (Variables|Default|GetIsOpen)
        (CallFunction|CloseDoor)
        (if (Variables|Default|GetIsUp)
          (CallFunction|MoveElevatorDown)
          (else
            (CallFunction|MoveElevatorUp)))
        (else
          (CallFunction|OpenDoor))))))

(fn ConstructionScript)