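; BP_Ring2 is a ring structure for the navigation map environment whose LED lights can fade in.
; The construction script caches the point lights parented to the LedLightsRing2 component into an array.
; FadeInLedlightsRing2, gated by the PlayFadeInRing2 flag, plays a timeline that drives those lights' intensity and the Emission material parameter on LedLightsRing2 together.
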(event Custom|FadeIn%20Led%20lights%20Ring2
  (if (Variables|Default|GetPlay%20FadeIn%20Ring%202)
    (bind (_direction _lights_components_intensity _emission_value) (Timeline|Timeline_0 Play)
      (:Update
        (for _array_element (Variables|Default|GetLed%20Lights%20Components)
          (Rendering|Components|Light|SetIntensity _array_element _lights_components_intensity)
          (Rendering|Material|SetScalarParameterValueonMaterials (Variables|Default|GetLedLights_Ring2) "Emission" _emission_value))))))

(event EventBeginPlay)

(event Collision|EventActorBeginOverlap
  (params (OtherActor :type Actor%20Object%20Reference)))

(event EventTick
  (params (DeltaSeconds :type Float%20%28single-precision%29)))

(fn ConstructionScript
  (for _array_element (Components|GetChildrenComponents (Variables|Default|GetLedLights_Ring2) false)
    (bind _aspoint_light_component (Utilities|Casting|CastToPointLightComponent _array_element))
    (Utilities|Array|Add (Variables|Default|GetLed%20Lights%20Components) _aspoint_light_component)))