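; Ship tile that runs a hammer pickup objective and opens one of five gated exits.
; Pickups spawn one at a time within a distance band of the player until the series completes, then HUD, game mode and chosen transporter advance play.
; MakeVisible matches a gate transform by near-equality to reveal its exit, remove its glass and select its transporter.
; Construction script restyles every BP_PickUpActor and sets each transporter's three path points.
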(event Custom|GotPickupActor
  (params (ActorPicked :type BP%20Pick%20Up%20Actor%20Object%20Reference))
  (bind _returnvalue (Game|GetPlayerController 0))
  (bind _transportertoshow (Variables|Default|GetTransporterToShow))
  (bind _returnvalue_2 (Utilities|Array|RemoveItem (Variables|Default|GetPickupActors) ActorPicked))
  (if _returnvalue_2
    (Actor|DestroyActor ActorPicked))
  (if (>= (Variables|Default|GetSeries) (Variables|Default|GetTotalSeries))
    (bind _asbp_hud (Utilities|Casting|CastToBP_HUD (HUD|GetHUD _returnvalue)))
    (Default|ShowTileDone _asbp_hud)
    (bind _ashg_bp_hynmers_character (Utilities|Casting|CastToHG_BP_HynmersCharacter (Pawn|GetControlledPawn _returnvalue)))
    (Variables|/Script/HynmersGame.HynmersCharacter|SetbCanMoveWithController _ashg_bp_hynmers_character true)
    (bind _ashg_bp_game_mode (Utilities|Casting|CastToHG_BP_GameMode (Game|GetGameMode)))
    (Default|ShowNextTile _ashg_bp_game_mode)
    (Utilities|IsValid _transportertoshow
      (:Is%20Valid
        (Default|Show _transportertoshow)))
    (else
      (CallFunction|SpawnPickupActor))))

(event Custom|InitAvailableGates
  (bind _output_get (Variables|Default|SetAvailableGates (Variables|Default|GetGates)))
  (Utilities|Array|Shuffle _output_get))

(event Custom|SpawnPickupActor
  (bind _returnvalue (Game|GetPlayerController 0))
  (Utilities|Array|Shuffle (Variables|Default|GetPickupActors))
  (bind _array_element (Utilities|Array|ForEachLoopwithBreak (Variables|Default|GetPickupActors) :!label _label)
    (:LoopBody
      (if (and (>= (Transformation|GetHorizontalDistanceTo _array_element (Game|Player|GetPlayerPawn 0)) (Variables|Default|GetMinDistance)) (<= (Transformation|GetHorizontalDistanceTo _array_element (Game|Player|GetPlayerPawn 0)) (Variables|Default|GetMaxDistance)))
        (Variables|Default|SetActorToSpawn _array_element)
        (goto _label Break)))
    (:Completed
      (Utilities|IsValid (Variables|Default|GetActorToSpawn)
        (:Is%20Valid
          (Utilities|FlowControl|Sequence
            (:then_0
              (Rendering|SetActorHiddenInGame (Variables|Default|GetActorToSpawn) false)
              (Collision|SetCollisionEnabled (Variables|/Game/Hynmers/Mechanics/BP_PickUpActor.BP_PickUpActor_C|GetSphere (Variables|Default|GetActorToSpawn)) "QueryOnly")
              (Development|SetHiddeninGame (Variables|/Game/Hynmers/Mechanics/BP_PickUpActor.BP_PickUpActor_C|GetStaticMesh (Variables|Default|GetActorToSpawn)) false false)
              (Components|Activation|SetActive (Variables|/Game/Hynmers/Mechanics/BP_PickUpActor.BP_PickUpActor_C|GetParticleSystem (Variables|Default|GetActorToSpawn)) true true)
              (Development|SetHiddeninGame (Variables|/Game/Hynmers/Mechanics/BP_PickUpActor.BP_PickUpActor_C|GetParticleSystem (Variables|Default|GetActorToSpawn)) false false)
              (Rendering|SetVisibility (Variables|/Game/Hynmers/Mechanics/BP_PickUpActor.BP_PickUpActor_C|GetParticleSystem (Variables|Default|GetActorToSpawn)) true false))
            (:then_1
              (bind _ashynmers_player_controller (Utilities|Casting|CastToHynmersPlayerController _returnvalue))
              (Class|HynmersPlayerController|SetCurrentPickUpActor _ashynmers_player_controller (Transformation|GetDistanceTo (Pawn|GetControlledPawn _returnvalue) (Variables|Default|GetActorToSpawn)) (Variables|Default|GetRepetitions)))))))))

(event Custom|ActivePlay
  (CallFunction|GetAllPickupActors))

(event Custom|GetAllPickupActors
  (bind _outactors (Actor|GetAllActorsOfClass "/Game/Hynmers/Mechanics/BP_PickUpActor.BP_PickUpActor_C"))
  (Variables|Default|SetPickupActors _outactors)
  (CallFunction|SpawnPickupActor))

(event Custom|LocateArrow
  (bind _availablegates (Variables|Default|GetAvailableGates))
  (Transformation|SetWorldTransform (Variables|Default|GetArrow) (Utilities|Array|Get(acopy) _availablegates (Math|Random|RandomIntegerinRange 0 (- (Utilities|Array|Length _availablegates) 1))) false true))

(fn ConstructionScript
  (Utilities|FlowControl|Sequence
    (:then_0
      (bind _outactors (Actor|GetAllActorsOfClass "/Game/Hynmers/Mechanics/BP_PickUpActor.BP_PickUpActor_C"))
      (for _array_element _outactors
        (Components|StaticMesh|SetStaticMesh (Variables|/Game/Hynmers/Mechanics/BP_PickUpActor.BP_PickUpActor_C|GetStaticMesh _array_element) "/Game/ToolShedVOL1/Meshes/SM_Hammer_01.SM_Hammer_01")
        (Effects|Components|ParticleSystem|SetTemplate (Variables|/Game/Hynmers/Mechanics/BP_PickUpActor.BP_PickUpActor_C|GetParticleSystem _array_element) "/Game/Hynmers/VFX/P_Circle_ChargeUp.P_Circle_ChargeUp")))
    (:then_1
      (Utilities|SetTransporterTransforms (Variables|Default|GetPawnTransporter1) (Math|Transform|MakeTransform "0, 0,56.000000" "0,180.000000, 0") (Math|Transform|MakeTransform "0, 0,318.000000" "0,180.000000, 0") (Math|Transform|MakeTransform "-635.000000,-72.000000,395.000000" "20.000000,180.000000,0.000000" "1.000000,1,1")
        (:Done
          (Utilities|SetTransporterTransforms (Variables|Default|GetPawnTransporter2) (Math|Transform|MakeTransform "0, 0,269.000000") (Math|Transform|MakeTransform "40.000000,0.000000,598.000000" "0.000000,-10.000000,0.000000") (Math|Transform|MakeTransform "798.000000,-120.000000,589.000000" "0, 0,0.000000")
            (:Done
              (Utilities|SetTransporterTransforms (Variables|Default|GetPawnTransporter3) (Math|Transform|MakeTransform "-26.000000,0.000000,163.000000" "0.000000,0.000000,0.000000") (Math|Transform|MakeTransform "97.000000,0.000000,573.000000") (Math|Transform|MakeTransform "946.000000,0.000000,585.000000" "15.000000, 0,0.000000" "1,1.000000,1")
                (:Done
                  (Utilities|SetTransporterTransforms (Variables|Default|GetPawnTransporter4) (Math|Transform|MakeTransform "0.000000,0.000000,279.000000" "0, 0,0.000000") (Math|Transform|MakeTransform "357.000000,0.000000,320.000000" "15.000000,-20.000000,0.000000") (Math|Transform|MakeTransform "996.000000,-331.000000,575.000000")
                    (:Done
                      (Utilities|SetTransporterTransforms (Variables|Default|GetPawnTransporter5) (Math|Transform|MakeTransform "0.000000, 0,98.000000" "0.000000,30.000000,0.000000") (Math|Transform|MakeTransform "0.000000,172.000000,420.000000" "0.000000,20.000000,0.000000") (Math|Transform|MakeTransform "838.000000,176.000000,690.000000" "25.000000, 0,0.000000")))))))))))))

(fn MakeVisible
  (params (Gate :type Transform))
  (bind _gates (Variables|Default|GetGates))
  (bind _found (CallFunction|ArrayFind _gates Gate))
  (if (CallFunction|ArrayContains (Variables|Default|GetGates) Gate)
    (bind _asbp_pawn_transporter (Utilities|Casting|CastToBP_PawnTransporter (Variables|/Script/Engine.ChildActorComponent|GetChildActor (Utilities|Select :Index _found :Option%200 (Variables|Default|GetPawnTransporter1) :Option%201 (Variables|Default|GetPawnTransporter2) :Option%202 (Variables|Default|GetPawnTransporter3) :Option%203 (Variables|Default|GetPawnTransporter4) :Option%204 (Variables|Default|GetPawnTransporter5)))))
    (Variables|Default|SetTransporterToShow _asbp_pawn_transporter)
    (Development|SetHiddeninGame (Utilities|Select :Index _found :Option%200 (Variables|Default|GetExit1) :Option%201 (Variables|Default|GetExit2) :Option%202 (Variables|Default|GetExit3) :Option%203 (Variables|Default|GetExit4) :Option%204 (Variables|Default|GetExit5)) false false)
    (Components|DestroyComponent (Utilities|Select :Index _found :Option%200 (Variables|Default|GetGlass1) :Option%201 (Variables|Default|GetGlass2) :Option%202 (Variables|Default|GetGlass3) :Option%203 (Variables|Default|GetGlass4) :Option%204 (Variables|Default|GetGlass5)))))

(fn ArrayContains
  (params (Transforms :type Array%20of%20Transforms) (Transform :type Transform))
  (bind _array_element (Utilities|Array|ForEachLoopwithBreak Transforms)
    (:LoopBody
      (if (Class|KismetMathLibrary|NearlyEqualTransformTransform _array_element Transform 0.0001 0.0001 0.0001)
        (return true)))
    (:Completed
      (return false))))

(fn ArrayFind
  (params (Transforms :type Array%20of%20Transforms) (Transform :type Transform))
  (bind (_array_element _array_index) (Utilities|Array|ForEachLoopwithBreak Transforms)
    (:LoopBody
      (if (Class|KismetMathLibrary|NearlyEqualTransformTransform _array_element Transform 0.0001 0.0001 0.0001)
        (return _array_index)))
    (:Completed
      (return -1))))