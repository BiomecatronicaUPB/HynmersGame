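; BP_Machines is a Hynmers game tile that runs an exercise as a sequence of pickups, with series, repetitions and limits taken from game session info.
; Player overlap collects child pickup actors, then reveals a shuffled one within a distance range and passes its distance and repetitions to the player controller.
; Each pickup triggers the next until the series total is reached, when the tile completes, restores movement and shows the next tile.
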(event OnComponentBeginOverlap(Box)
  (params (OverlappedComponent :type Primitive%20Component%20Object%20Reference) (OtherActor :type Actor%20Object%20Reference) (OtherComp :type Primitive%20Component%20Object%20Reference) (OtherBodyIndex :type Integer) (bFromSweep :type Boolean) (SweepResult :type Hit%20Result%20Structure%20%28by%20ref%29))
  (Utilities|Casting|CastToHG_BP_HynmersCharacter OtherActor)
  (CallFunction|ActivePlay))

(event Custom|GotPickupActor
  (params (ActorPicked :type BP%20Pick%20Up%20Actor%20Object%20Reference))
  (bind _returnvalue (Game|GetPlayerController 0))
  (bind _returnvalue_2 (Utilities|Array|RemoveItem (Variables|Default|GetPickupActors) ActorPicked))
  (if _returnvalue_2
    (Actor|DestroyActor ActorPicked))
  (if (>= (Variables|Default|GetSeries) (Variables|Default|GetTotalSeries))
    (bind _asbp_hud (Utilities|Casting|CastToBP_HUD (HUD|GetHUD _returnvalue)))
    (Default|ShowTileDone _asbp_hud)
    (bind _ashg_bp_hynmers_character (Utilities|Casting|CastToHG_BP_HynmersCharacter (Pawn|GetControlledPawn _returnvalue)))
    (Variables|/Script/HynmersGame.HynmersCharacter|SetbCanMoveWithController _ashg_bp_hynmers_character true)
    (bind _ashg_bp_game_mode (Utilities|Casting|CastToHG_BP_GameMode (Game|GetGameMode)))
    (Default|ShowNextTile _ashg_bp_game_mode)
    (Variables|Default|SetbCompleted true)
    (bind _outactors (Actor|GetAllActorsOfClass "/Script/Engine.PhysicsVolume"))
    (if (Utilities|Array|IsValidIndex _outactors)
      (Actor|DestroyActor (Utilities|Array|Get(acopy) _outactors)))
    (else
      (CallFunction|SpawnPickupActor))))

(event Custom|SpawnPickupActor
  (bind _returnvalue (Game|GetPlayerController 0))
  (Utilities|Array|Shuffle (Variables|Default|GetPickupActors))
  (bind _array_element (Utilities|Array|ForEachLoopwithBreak (Variables|Default|GetPickupActors) :!label _label)
    (:LoopBody
      (if (and (>= (Transformation|GetHorizontalDistanceTo _array_element (Game|Player|GetPlayerPawn 0)) (Variables|Default|GetMinDistance)) (<= (Transformation|GetHorizontalDistanceTo _array_element (Game|Player|GetPlayerPawn 0)) (Variables|Default|GetMaxDistance)))
        (Variables|Default|SetActorToSpawn _array_element)
        (goto _label Break)))
    (:Completed
      (Utilities|IsValid (Variables|Default|GetActorToSpawn)
        (:Is%20Valid
          (Utilities|FlowControl|Sequence
            (:then_0
              (Rendering|SetActorHiddenInGame (Variables|Default|GetActorToSpawn) false)
              (Collision|SetCollisionEnabled (Variables|/Game/Hynmers/Mechanics/BP_PickUpActor.BP_PickUpActor_C|GetSphere (Variables|Default|GetActorToSpawn)) "QueryOnly")
              (Components|Activation|SetActive (Variables|/Game/Hynmers/Mechanics/BP_PickUpActor.BP_PickUpActor_C|GetParticleSystem (Variables|Default|GetActorToSpawn)) true true)
              (Development|SetHiddeninGame (Variables|/Game/Hynmers/Mechanics/BP_PickUpActor.BP_PickUpActor_C|GetParticleSystem (Variables|Default|GetActorToSpawn)) false false)
              (Rendering|SetVisibility (Variables|/Game/Hynmers/Mechanics/BP_PickUpActor.BP_PickUpActor_C|GetParticleSystem (Variables|Default|GetActorToSpawn)) true false))
            (:then_1
              (bind _ashynmers_player_controller (Utilities|Casting|CastToHynmersPlayerController _returnvalue))
              (Class|HynmersPlayerController|SetCurrentPickUpActor _ashynmers_player_controller (Transformation|GetDistanceTo (Pawn|GetControlledPawn _returnvalue) (Variables|Default|GetActorToSpawn)) (Variables|Default|GetRepetitions)))))))))

(event Custom|ActivePlay
  (if (not (Variables|Default|GetbCompleted))
    (CallFunction|GetAllPickupActors)))

(event Custom|GetAllPickupActors
  (bind _list (CallFunction|GetAllPickUpChildActor))
  (Variables|Default|SetPickupActors _list)
  (CallFunction|SpawnPickupActor))

(event EventBeginPlay)

(event Collision|EventActorBeginOverlap
  (params (OtherActor :type Actor%20Object%20Reference)))

(event EventTick
  (params (DeltaSeconds :type Float%20%28single-precision%29)))

(event EventInitParameters
  (params (GameSessionInfo :type Array%20of%20Session%20Info%20Structures))
  (bind _array_element (Utilities|Array|ForEachLoopwithBreak GameSessionInfo :!label _label)
    (:LoopBody
      (if (== (.ExerciseIndex (Utilities|Struct|BreakSessionInfo _array_element)) (Math|Conversions|ToInteger(Byte) (Variables|Default|GetTileType)))
        (Variables|Default|SetTotalSeries (.Series (Utilities|Struct|BreakSessionInfo _array_element)))
        (Variables|Default|SetRepetitions (.Repetitions (Utilities|Struct|BreakSessionInfo _array_element)))
        (Variables|Default|SetUpperLimits (.UpperLimits (Utilities|Struct|BreakSessionInfo _array_element)))
        (Variables|Default|SetLowerLimits (.LowerLimits (Utilities|Struct|BreakSessionInfo _array_element)))
        (goto _label Break)))))

(fn ConstructionScript)

(fn GetAllPickUpChildActor
  (for _array_element (Actor|GetAllChildActors true)
    (bind _asbp_pick_up_actor (Utilities|Casting|CastToBP_PickUpActor _array_element))
    (Utilities|Array|Add (LocalVariables|GetChildActors) _asbp_pick_up_actor))
  (return (LocalVariables|GetChildActors)))