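; Ship tile for the Hynmers game that runs a pickup exercise, with series and repetitions set from the session info for its tile type.
; It reveals a random pickup within a distance band of the player and passes it to the controller.
; Completing all series updates the HUD, restores movement, requests the next tile and shows the selected transporter.
; MakeVisible matches a gate transform to one of five exits, whose transporter paths are set at construction.
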(event Custom|GotPickupActor
  (params (ActorPicked :type BP%20Pick%20Up%20Actor%20Object%20Reference))
  (bind _returnvalue (Game|GetPlayerController 0))
  (bind _transportertoshow (Variables|Default|GetTransporterToShow))
  (bind _returnvalue_2 (Utilities|Array|RemoveItem (Variables|Default|GetPickupActors) ActorPicked))
  (if _returnvalue_2
    (Actor|DestroyActor ActorPicked))
  (if (>= (Variables|Default|GetSeries) (Variables|Default|GetTotalSeries))
    (bind _asbp_hud (Utilities|Casting|CastToBP_HUD (HUD|GetHUD _returnvalue)))
    (Default|ShowTileDone _asbp_hud)
    (bind _ashg_bp_hynmers_character (Utilities|Casting|CastToHG_BP_HynmersCharacter (Pawn|GetControlledPawn _returnvalue)))
    (Variables|/Script/HynmersGame.HynmersCharacter|SetbCanMoveWithController _ashg_bp_hynmers_character true)
    (bind _ashg_bp_game_mode (Utilities|Casting|CastToHG_BP_GameMode (Game|GetGameMode)))
    (Default|ShowNextTile _ashg_bp_game_mode)
    (Utilities|IsValid _transportertoshow
      (:Is%20Valid
        (Default|Show _transportertoshow)))
    (else
      (CallFunction|SpawnPickupActor))))

(event Custom|InitAvailableGates
  (bind _output_get (Variables|Default|SetAvailableGates (Variables|Default|GetGates)))
  (Utilities|Array|Shuffle _output_get))

(event Custom|SpawnPickupActor
  (bind _returnvalue (Game|GetPlayerController 0))
  (Utilities|Array|Shuffle (Variables|Default|GetPickupActors))
  (bind _array_element (Utilities|Array|ForEachLoopwithBreak (Variables|Default|GetPickupActors) :!label _label)
    (:LoopBody
      (if (and (>= (Transformation|GetHorizontalDistanceTo _array_element (Game|Player|GetPlayerPawn 0)) (Variables|Default|GetMinDistance)) (<= (Transformation|GetHorizontalDistanceTo _array_element (Game|Player|GetPlayerPawn 0)) (Variables|Default|GetMaxDistance)))
        (Variables|Default|SetActorToSpawn _array_element)
        (goto _label Break)))
    (:Completed
      (Utilities|IsValid (Variables|Default|GetActorToSpawn)
        (:Is%20Valid
          (Utilities|FlowControl|Sequence
            (:then_0
              (Rendering|SetActorHiddenInGame (Variables|Default|GetActorToSpawn) false)
              (Collision|SetCollisionEnabled (Variables|/Game/Hynmers/Mechanics/BP_PickUpActor.BP_PickUpActor_C|GetSphere (Variables|Default|GetActorToSpawn)) "QueryOnly")
              (Components|Activation|SetActive (Variables|/Game/Hynmers/Mechanics/BP_PickUpActor.BP_PickUpActor_C|GetParticleSystem (Variables|Default|GetActorToSpawn)) true true)
              (Development|SetHiddeninGame (Variables|/Game/Hynmers/Mechanics/BP_PickUpActor.BP_PickUpActor_C|GetParticleSystem (Variables|Default|GetActorToSpawn)) false false)
              (Rendering|SetVisibility (Variables|/Game/Hynmers/Mechanics/BP_PickUpActor.BP_PickUpActor_C|GetParticleSystem (Variables|Default|GetActorToSpawn)) true false))
            (:then_1
              (bind _ashynmers_player_controller (Utilities|Casting|CastToHynmersPlayerController _returnvalue))
              (Class|HynmersPlayerController|SetCurrentPickUpActor _ashynmers_player_controller (Transformation|GetDistanceTo (Pawn|GetControlledPawn _returnvalue) (Variables|Default|GetActorToSpawn)) (Variables|Default|GetRepetitions)))))))))

(event Custom|ActivePlay
  (CallFunction|GetAllPickupActors)
  (bind _ashg_bp_hynmers_character (Utilities|Casting|CastToHG_BP_HynmersCharacter (Game|Player|GetPlayerPawn 0)))
  (Variables|/Script/HynmersGame.HynmersCharacter|SetCurrentTile _ashg_bp_hynmers_character self))

(event Custom|GetAllPickupActors
  (bind _list (CallFunction|GetAllPickUpChildActor))
  (Variables|Default|SetPickupActors _list)
  (CallFunction|SpawnPickupActor))

(event Custom|LocateArrow
  (bind _availablegates (Variables|Default|GetAvailableGates))
  (Transformation|SetWorldTransform (Variables|Default|GetArrow) (Utilities|Array|Get(acopy) _availablegates (Math|Random|RandomIntegerinRange 0 (- (Utilities|Array|Length _availablegates) 1))) false true))

(event EventInitParameters
  (params (GameSessionInfo :type Array%20of%20Session%20Info%20Structures))
  (bind _array_element (Utilities|Array|ForEachLoopwithBreak GameSessionInfo :!label _label)
    (:LoopBody
      (if (== (.ExerciseIndex (Utilities|Struct|BreakSessionInfo _array_element)) (Math|Conversions|ToInteger(Byte) (Variables|Default|GetTileType)))
        (Variables|Default|SetTotalSeries (.Series (Utilities|Struct|BreakSessionInfo _array_element)))
        (Variables|Default|SetRepetitions (.Repetitions (Utilities|Struct|BreakSessionInfo _array_element)))
        (Variables|Default|SetUpperLimits (.UpperLimits (Utilities|Struct|BreakSessionInfo _array_element)))
        (Variables|Default|SetLowerLimits (.LowerLimits (Utilities|Struct|BreakSessionInfo _array_element)))
        (goto _label Break)))))

(fn ConstructionScript
  (Utilities|FlowControl|Sequence
    (:then_0
      (bind _list (CallFunction|GetAllPickUpChildActor))
      (for _array_element _list
        (Collision|SetCollisionEnabled (Variables|/Game/Hynmers/Mechanics/BP_PickUpActor.BP_PickUpActor_C|GetSphere _array_element) "NoCollision")))
    (:then_1
      (Utilities|SetTransporterTransforms (Variables|Default|GetPawnTransporter1) (Math|Transform|MakeTransform "0, 0,56.000000") (Math|Transform|MakeTransform "0, 0,318.000000") (Math|Transform|MakeTransform "635.000000,-72.000000,395.000000" "20.000000,0.000000,0.000000")
        (:Done
          (Utilities|SetTransporterTransforms (Variables|Default|GetPawnTransporter2) (Math|Transform|MakeTransform "0, 0,269.000000") (Math|Transform|MakeTransform "40.000000,0.000000,598.000000" "0.000000,-10.000000,0.000000") (Math|Transform|MakeTransform "798.000000,-120.000000,589.000000")
            (:Done
              (Utilities|SetTransporterTransforms (Variables|Default|GetPawnTransporter3) (Math|Transform|MakeTransform "-26.000000,0.000000,163.000000") (Math|Transform|MakeTransform "97.000000,0.000000,573.000000") (Math|Transform|MakeTransform "946.000000,0.000000,585.000000" "15.000000, 0,0.000000")
                (:Done
                  (Utilities|SetTransporterTransforms (Variables|Default|GetPawnTransporter4) (Math|Transform|MakeTransform "0.000000,0.000000,279.000000") (Math|Transform|MakeTransform "357.000000,0.000000,320.000000" "15.000000,-20.000000,0.000000") (Math|Transform|MakeTransform "996.000000,-331.000000,575.000000")
                    (:Done
                      (Utilities|SetTransporterTransforms (Variables|Default|GetPawnTransporter5) (Math|Transform|MakeTransform "0.000000, 0,98.000000" "0.000000,30.000000,0.000000") (Math|Transform|MakeTransform "0.000000,172.000000,420.000000" "0.000000,20.000000,0.000000") (Math|Transform|MakeTransform "838.000000,176.000000,690.000000" "25.000000, 0,0.000000")))))))))))))

(fn MakeVisible
  (params (Gate :type Transform))
  (bind _gates (Variables|Default|GetGates))
  (bind _found (CallFunction|ArrayFind _gates Gate))
  (if (CallFunction|ArrayContains (Variables|Default|GetGates) Gate)
    (bind _asbp_pawn_transporter (Utilities|Casting|CastToBP_PawnTransporter (Variables|/Script/Engine.ChildActorComponent|GetChildActor (Utilities|Select :Index _found :Option%200 (Variables|Default|GetPawnTransporter1) :Option%201 (Variables|Default|GetPawnTransporter2) :Option%202 (Variables|Default|GetPawnTransporter3) :Option%203 (Variables|Default|GetPawnTransporter4) :Option%204 (Variables|Default|GetPawnTransporter5)))))
    (Variables|Default|SetTransporterToShow _asbp_pawn_transporter)
    (Development|SetHiddeninGame (Utilities|Select :Index _found :Option%200 (Variables|Default|GetExit1) :Option%201 (Variables|Default|GetExit2) :Option%202 (Variables|Default|GetExit3) :Option%203 (Variables|Default|GetExit4) :Option%204 (Variables|Default|GetExit5)) false false)
    (Components|DestroyComponent (Utilities|Select :Index _found :Option%200 (Variables|Default|GetGlass1) :Option%201 (Variables|Default|GetGlass2) :Option%202 (Variables|Default|GetGlass3) :Option%203 (Variables|Default|GetGlass4) :Option%204 (Variables|Default|GetGlass5)))))

(fn ArrayContains
  (params (Transforms :type Array%20of%20Transforms) (Transform :type Transform))
  (bind _array_element (Utilities|Array|ForEachLoopwithBreak Transforms)
    (:LoopBody
      (if (Class|KismetMathLibrary|NearlyEqualTransformTransform _array_element Transform 0.0001 0.0001 0.0001)
        (return true)))
    (:Completed
      (return false))))

(fn ArrayFind
  (params (Transforms :type Array%20of%20Transforms) (Transform :type Transform))
  (bind (_array_element _array_index) (Utilities|Array|ForEachLoopwithBreak Transforms)
    (:LoopBody
      (if (Class|KismetMathLibrary|NearlyEqualTransformTransform _array_element Transform 0.0001 0.0001 0.0001)
        (return _array_index)))
    (:Completed
      (return -1))))

(fn GetAllPickUpChildActor
  (for _array_element (Actor|GetAllChildActors true)
    (bind _asbp_pick_up_actor (Utilities|Casting|CastToBP_PickUpActor _array_element))
    (Utilities|Array|Add (LocalVariables|GetChildActors) _asbp_pick_up_actor))
  (return (LocalVariables|GetChildActors)))