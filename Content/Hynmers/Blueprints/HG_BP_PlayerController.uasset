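; Player controller Blueprint for Hynmers that handles the quit and interact inputs.
; The Quit action exits the game.
; The Interact action casts the controlled pawn to the Hynmers character, gathers its overlapping interactive actors, and calls Interact on them, passing the pawn as the argument.
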(event EventBeginPlay)

(event EventTick
  (params (DeltaSeconds :type Float%20%28single-precision%29)))

(event Input|ActionEvents|InputActionQuit
  (params (Key :type Key%20Structure))
  (:Pressed
    (Game|QuitGame self "Quit")))

(event Input|ActionEvents|InputActionInteract
  (params (Key :type Key%20Structure))
  (:Pressed
    (bind _ashg_bp_hynmers_character (Utilities|Casting|CastToHG_BP_HynmersCharacter (Pawn|GetControlledPawn)))
    (if (> (Utilities|Array|Length (Collision|GetOverlappingActors _ashg_bp_hynmers_character "/Script/HynmersGame.HynmersInteractiveActor" :!class /Script/Engine.Actor)) 0)
      (for _array_element (Collision|GetOverlappingActors _ashg_bp_hynmers_character "/Script/HynmersGame.HynmersInteractiveActor" :!class /Script/Engine.Actor)
        (bind _ashynmers_interactive_actor (Utilities|Casting|CastToHynmersInteractiveActor _array_element))
        (Class|HynmersInteractiveActor|Interact _ashynmers_interactive_actor (Pawn|GetControlledPawn))))))

(fn ConstructionScript)